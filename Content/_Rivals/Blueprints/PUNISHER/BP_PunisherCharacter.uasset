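; BP_PunisherCharacter is the playable Punisher hero blueprint, mapping player input to the character's weapon and ability actions.
; Primary attack branches on the active weapon, firing weapon 1 on press and release or triggering a shotgun attack otherwise, and number keys switch between the two.
; Other inputs call smoke impact, reload, grapple hook, and a turret action that deploys or ends based on its active status.
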(event Input|EnhancedActionEvents|EnhancedInputActionIA_RMB
  (params (ActionValue :type Boolean) (ElapsedSeconds :type Float%20%28double-precision%29) (TriggeredSeconds :type Float%20%28double-precision%29) (InputAction :type Input%20Action%20Object%20Reference :default "/Game/ThirdPerson/Input/Actions/IA_RMB.IA_RMB"))
  (:Started
    (Class|PunisherCharacter|RMBSmokeImpact)))

(event Input|EnhancedActionEvents|EnhancedInputActionIA_PrimaryAttack
  (params (ActionValue :type Boolean) (ElapsedSeconds :type Float%20%28double-precision%29) (TriggeredSeconds :type Float%20%28double-precision%29) (InputAction :type Input%20Action%20Object%20Reference :default "/Game/ThirdPerson/Input/Actions/IA_PrimaryAttack.IA_PrimaryAttack"))
  (:Started
    (if (== (Class|PunisherCharacter|GetActiveWeapon) 1)
      (Class|PunisherCharacter|LMBFireBtnPressed)
      (else
        (Class|PunisherCharacter|LMBShotGunAttack))))
  (:Completed
    (Class|PunisherCharacter|LMBFireBtnReleased)))

(event Input|EnhancedActionEvents|EnhancedInputActionIA_Reload
  (params (ActionValue :type Boolean) (ElapsedSeconds :type Float%20%28double-precision%29) (TriggeredSeconds :type Float%20%28double-precision%29) (InputAction :type Input%20Action%20Object%20Reference :default "/Game/ThirdPerson/Input/Actions/IA_Reload.IA_Reload"))
  (:Started
    (Class|PunisherCharacter|ReloadGunWrapper)))

(event Input|EnhancedActionEvents|EnhancedInputActionIA_Shift
  (params (ActionValue :type Boolean) (ElapsedSeconds :type Float%20%28double-precision%29) (TriggeredSeconds :type Float%20%28double-precision%29) (InputAction :type Input%20Action%20Object%20Reference :default "/Game/ThirdPerson/Input/Actions/IA_Shift.IA_Shift"))
  (:Started
    (Class|PunisherCharacter|ShiftGrappleHook)))

(event Input|KeyboardEvents|1
  (params (Key :type Key%20Structure :default "None"))
  (:Pressed
    (Class|PunisherCharacter|SwitchWeapon 1)))

(event Input|KeyboardEvents|2
  (params (Key :type Key%20Structure :default "None"))
  (:Pressed
    (Class|PunisherCharacter|SwitchWeapon 2)))

(event Input|KeyboardEvents|E
  (params (Key :type Key%20Structure :default "None"))
  (:Pressed
    (if (Class|PunisherCharacter|GetTurretActiveStatus)
      (Class|PunisherCharacter|PreEndTurretAction)
      (else
        (Class|PunisherCharacter|ETurretButton)))))

(fn ConstructionScript)